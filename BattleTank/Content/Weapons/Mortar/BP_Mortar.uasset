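; BP_Mortar is a player-controlled mortar weapon that aims and fires through a MortarAiming component.
; On BeginPlay it passes its barrel and dome turret to that component, which also handles the fire input.
; Aim axes rotate an azimuth gimbal for yaw and a spring arm for pitch, scaled by delta time, steering the view separately from the barrel.
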(event EventBeginPlay
  (Class|TankAimingComponent|Initialise (Variables|Default|GetMortarAiming) (Variables|Default|GetBarrel) (Variables|Default|GetDome)))

(event Input|ActionEvents|InputActionFire
  (params (Key :type Key%20Structure :default "AnyKey"))
  ;[1 1 1] Input Bindings
  (:Pressed
    (Class|TankAimingComponent|Fire (Variables|Default|GetMortarAiming))))

(event Input|AxisEvents|InputAxisAimAzimuth
  (params (AxisValue :type Float%20%28single-precision%29))
  ;[1 1 1] Input Bindings
  ;;[1 1 1] Left & Right View Controls
  (Transformation|AddLocalRotation (Variables|Default|GetAzimuth%20Gimbal) (Math|Rotator|MakeRotator 0.0 0.0 (* AxisValue (Utilities|Time|GetWorldDeltaSeconds) 1e+02)) false false))

(event Input|AxisEvents|InputAxisAimElevation
  (params (AxisValue :type Float%20%28single-precision%29))
  ;[1 1 1] Input Bindings
  ;;[1 1 1] Up & Down View Controls
  (Transformation|AddLocalRotation (Variables|Default|GetSpringArm) (Math|Rotator|MakeRotator 0.0 (* AxisValue (Utilities|Time|GetWorldDeltaSeconds) 1e+02) 0.0) false false))

(fn ConstructionScript)