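; BP_Tank is a controllable tank that drives on tracks, aims with an orbiting camera, fires, and shows a health bar.
; On BeginPlay it hands the barrel, turret and tracks to TankAiming and TankMovement, then gives the health bar widget a reference to itself.
; Input forwards drive, turn and fire to those components, rotates the azimuth gimbal and spring arm at frame-rate-independent speed, and toggles first- and third-person cameras.
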(event EventBeginPlay
  (Class|TankAimingComponent|Initialise (Variables|Default|GetTankAiming) (Variables|Default|GetBarrel) (Variables|Default|GetTurret))
  (Class|TankMovementComponent|Initialise (Variables|Default|GetTankMovement) (Variables|Default|GetTrack_L) (Variables|Default|GetTrack_R))
  (CallFunction|InitialiseHealthBarWidget))

(event Input|ActionEvents|InputActionFire
  (params (Key :type Key%20Structure :default "AnyKey"))
  ;[1 1 1] Input Bindings
  (:Pressed
    (Class|TankAimingComponent|Fire (Variables|Default|GetTankAiming))))

(event Input|ActionEvents|InputActionChangeCamera
  (params (Key :type Key%20Structure :default "AnyKey"))
  ;[1 1 1] Camera Swap Controls
  (:Pressed
    (Components|Activation|ToggleActive (Variables|Default|Get1st%20Person))
    (Components|Activation|ToggleActive (Variables|Default|Get3rd%20Person))))

(event Input|AxisEvents|InputAxisAimAzimuth
  (params (AxisValue :type Float%20%28single-precision%29))
  ;[1 1 1] Input Bindings
  ;;[1 1 1] Left & Right View Controls
  (Transformation|AddLocalRotation (Variables|Default|GetAzimuth%20Gimbal) (Math|Rotator|MakeRotator 0.0 0.0 (* AxisValue (Utilities|Time|GetWorldDeltaSeconds) 1e+02)) false false))

(event Input|AxisEvents|InputAxisMoveForward
  (params (AxisValue :type Float%20%28single-precision%29))
  ;[1 1 1] Movement Input Bindings
  (Class|TankMovementComponent|IntendMoveForward (Variables|Default|GetTankMovement) AxisValue))

(event Input|AxisEvents|InputAxisTurnRight
  (params (AxisValue :type Float%20%28single-precision%29))
  ;[1 1 1] Movement Input Bindings
  (Class|TankMovementComponent|IntendTurnRight (Variables|Default|GetTankMovement) AxisValue))

(event Input|AxisEvents|InputAxisAimElevation
  (params (AxisValue :type Float%20%28single-precision%29))
  ;[1 1 1] Input Bindings
  ;;[1 1 1] Up & Down View Controls
  (Transformation|AddLocalRotation (Variables|Default|GetSpringArm) (Math|Rotator|MakeRotator 0.0 (* AxisValue (Utilities|Time|GetWorldDeltaSeconds) 1e+02) 0.0) false false))

(fn ConstructionScript)

(fn InitialiseHealthBarWidget
  (bind _asbp_health_bar (Utilities|Casting|CastToBP_HealthBar (UserInterface|GetUserWidgetObject (Variables|Default|GetHealth%20Bar%20Widget))))
  (Variables|/Game/UI/BP_HealthBar.BP_HealthBar_C|SetMyTank _asbp_health_bar self)
  (return))